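; Game mode for the Catapult game that runs the match flow from pregame through play to a win or end screen.
; On BeginPlay it shows the pregame widget, initializes and caches managers found through the I_Managers interface, then spawns and possesses the player pawn.
; Startgame hides the cursor, advances the state enum and shows the in-game HUD.
; EndGame shows the win screen only for a win in that state, otherwise the end screen.
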(event Custom|Init
  (bind _returnvalue (UserInterface|CreateWidget "/Game/Widgets/W_Pregame.W_Pregame_C"))
  (UserInterface|Viewport|AddtoPlayerScreen _returnvalue)
  (Variables|Default|SetGameStates "NewEnumerator0")
  (CallFunction|SetupManagers)
  (CallFunction|SpawnPlayer))

(event Custom|EndGame
  (params (Win :type Boolean))
  (if (and Win (Utilities|Enum|Equal(Enum) (Variables|Default|GetGameStates) "NewEnumerator1"))
    (Viewport|RemoveAllWidgets)
    (bind _returnvalue (UserInterface|CreateWidget "/Game/Widgets/W_WinGame.W_WinGame_C"))
    (UserInterface|Viewport|AddtoPlayerScreen _returnvalue)
    (else
      (Viewport|RemoveAllWidgets)
      (bind _returnvalue_2 (UserInterface|CreateWidget "/Game/Widgets/W_Endgame.W_Endgame_C"))
      (UserInterface|Viewport|AddtoPlayerScreen _returnvalue_2))))

(event Custom|Startgame
  (Viewport|RemoveAllWidgets)
  (Variables|/Script/Engine.PlayerController|SetbShowMouseCursor (Game|GetPlayerController 0) false)
  (Variables|Default|SetGameStates "NewEnumerator1")
  (bind _returnvalue (UserInterface|CreateWidget "/Game/Widgets/W_InGame.W_InGame_C"))
  (UserInterface|Viewport|AddtoPlayerScreen _returnvalue))

(event EventBeginPlay
  (CallFunction|Init))

(fn ConstructionScript)

(fn SpawnPlayer
  (bind _asc_player_controller (Utilities|Casting|CastToC_PlayerController (Game|GetPlayerController 0)))
  (bind _output_get (Variables|Default|SetPlayer _asc_player_controller))
  (bind _returnvalue (Game|SpawnActorfromClass "/Game/Base/P_PlayerPawn.P_PlayerPawn_C" (Variables|/Game/Base/C_PlayerController.C_PlayerController_C|GetSpawnPoint _output_get) "Undefined" 0 0))
  (bind _output_get_2 (Variables|/Game/Base/C_PlayerController.C_PlayerController_C|SetOwnedPawn (Variables|Default|GetPlayer) _returnvalue))
  (Default|Init (Variables|Default|GetPlayer))
  (Default|Init _output_get_2)
  (Pawn|Possess (Variables|Default|GetPlayer) _output_get_2)
  (return))

(fn SetupManagers
  (bind _outactors (Actor|GetAllActorswithInterface "/Game/I_Managers.I_Managers_C"))
  (for _array_element _outactors
    (Class|IManagers|Init(Message) _array_element)
    (bind _asbase_manager (Utilities|Casting|CastToBaseManager _array_element))
    (Utilities|Array|Add (LocalVariables|GetTempmanagers) _asbase_manager))
  (bind _output_get (Variables|Default|SetActiveManagers (LocalVariables|GetTempmanagers)))
  (return _output_get))